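; Strength-test puzzle actor: a button-mash minigame that awards the player a ticket once and requires the hammer to play.
; Its trigger overlap shows either the interact prompt or an alternate one if the hammer is missing, and IA_Action opens the progress HUD and signals the player's paused state.
; IA_PuzzleMash raises progress while a Timeline drains it; filling the bar deactivates the puzzle, and IA_PuzzleExit closes it early.
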(event `EnhancedInput|/Game/Input/Actions/IA_PuzzleMash`
  (params (ActionValue :type Boolean) (ElapsedSeconds :type "Float (double-precision)") (TriggeredSeconds :type "Float (double-precision)") (InputAction :type "InputAction Object Reference" :default "/Game/Input/Actions/IA_PuzzleMash.IA_PuzzleMash"))
  (:`Started`
    (if (`self.ispaused`)
      (bind _output_get (set `self.ProgressCurrent` (+ 5.0 (`self.ProgressCurrent`))))
      (bind _returnvalue (/ _output_get 100.0))
      (`ProgressBar.SetPercent` (`/Game/HUD/StrengthPuzzleHUD.ProgressBar` (`self.HUDref`)) _returnvalue)
      (if (>= _returnvalue 1.0)
        (bind _output_get_2 (set `self.ispaused` false))
        (`/Game/FirstPerson/Blueprints/BP_FirstPersonCharacter.gamePaused_Event` (`self.Player Ref`) _output_get_2)
        (`Widget.RemoveFromParent` (`self.HUDref`))
        (set `/Game/FirstPerson/Blueprints/BP_FirstPersonCharacter.Tickets` (+ 1.0 (`/Game/FirstPerson/Blueprints/BP_FirstPersonCharacter.Tickets` (`self.Player Ref`))) (`self.Player Ref`))
        (set `self.puzzle active` false)
        (`SceneComponent.SetVisibility` (`self.Interact Text`) false false)
        (set `self.Strength Puzzle` false)
        (`GameplayStatics.PlaySound2D` "/Game/Audio/universfield-video-game-bonus-323603.universfield-video-game-bonus-323603" 1.0 1.0 0.0 null null)))))

(event `EnhancedInput|/Game/Input/Actions/IA_Action`
  (params (ActionValue :type Boolean) (ElapsedSeconds :type "Float (double-precision)") (TriggeredSeconds :type "Float (double-precision)") (InputAction :type "InputAction Object Reference" :default "/Game/Input/Actions/IA_Action.IA_Action"))
  (:`Started`
    (if (`self.Strength Puzzle`)
      (if (not (`self.ispaused`))
        (bind _returnvalue (`|CreateWidget` "/Game/HUD/StrengthPuzzleHUD.StrengthPuzzleHUD_C"))
        (bind _output_get (set `self.HUDref` _returnvalue))
        (`UserWidget.AddToViewport` _output_get 0)
        (bind _output_get_2 (set `self.ispaused` true))
        (`/Game/FirstPerson/Blueprints/BP_FirstPersonCharacter.gamePaused_Event` (`self.Player Ref`) _output_get_2)
        (set `self.ProgressCurrent` 0.0)
        (bind (_direction _0) (`Timeline|Timeline` :!via `PlayFromStart`)
          (:`Update`
            (bind _returnvalue_2 (- (`self.ProgressCurrent`) _0))
            (if (<= _returnvalue_2 0.0)
              (set `self.ProgressCurrent` 0.0)
              (bind _output_get_3 (set `self.ProgressCurrent` _returnvalue_2))
              (`ProgressBar.SetPercent` (`/Game/HUD/StrengthPuzzleHUD.ProgressBar` (`self.HUDref`)) (/ _output_get_3 100.0))
              (else
                (bind _output_get_4 (set `self.ProgressCurrent` _returnvalue_2))
                (`ProgressBar.SetPercent` (`/Game/HUD/StrengthPuzzleHUD.ProgressBar` (`self.HUDref`)) (/ _output_get_4 100.0))))))))))

(event `self.ReceiveBeginPlay`
  (`self.EnableInput` (`GameplayStatics.GetPlayerController` 0)))

(event `EnhancedInput|/Game/Input/Actions/IA_PuzzleExit`
  (params (ActionValue :type Boolean) (ElapsedSeconds :type "Float (double-precision)") (TriggeredSeconds :type "Float (double-precision)") (InputAction :type "InputAction Object Reference" :default "/Game/Input/Actions/IA_PuzzleExit.IA_PuzzleExit"))
  (:`Started`
    (if (`self.ispaused`)
      (`Widget.RemoveFromParent` (`self.HUDref`))
      (bind _output_get (set `self.ispaused` false))
      (`/Game/FirstPerson/Blueprints/BP_FirstPersonCharacter.gamePaused_Event` (`self.Player Ref`) _output_get))))

(event `self.StrengthTrigger.OnComponentBeginOverlap`
  (params (OverlappedComponent :type "PrimitiveComponent Object Reference") (OtherActor :type "Actor Object Reference") (OtherComp :type "PrimitiveComponent Object Reference") (OtherBodyIndex :type Integer) (bFromSweep :type Boolean) (SweepResult :type "HitResult Structure (by ref)"))
  (bind _asbp_first_person_character (cast `/Game/FirstPerson/Blueprints/BP_FirstPersonCharacter` (`GameplayStatics.GetPlayerCharacter` 0)))
  (bind _output_get (set `self.Player Ref` _asbp_first_person_character))
  (if (`/Game/FirstPerson/Blueprints/BP_FirstPersonCharacter.Has Hammer` _output_get)
    (if (and (== _output_get OtherActor) (`self.puzzle active`))
      (`SceneComponent.SetVisibility` (`self.Interact Text`) true false)
      (set `self.Strength Puzzle` true))
    (else
      (`SceneComponent.SetVisibility` (`self.Interact Text1`) true false))))

(event `self.ReceiveTick`
  (params (DeltaSeconds :type "Float (single-precision)"))
  (if (`self.ispaused`)
    _))

(event `self.StrengthTrigger.OnComponentEndOverlap`
  (params (OverlappedComponent :type "PrimitiveComponent Object Reference") (OtherActor :type "Actor Object Reference") (OtherComp :type "PrimitiveComponent Object Reference") (OtherBodyIndex :type Integer))
  (bind _asbp_first_person_character (cast `/Game/FirstPerson/Blueprints/BP_FirstPersonCharacter` (`GameplayStatics.GetPlayerCharacter` 0)))
  (bind _output_get (set `self.Player Ref` _asbp_first_person_character))
  (if (== _output_get OtherActor)
    (`SceneComponent.SetVisibility` (`self.Interact Text`) false false)
    (`SceneComponent.SetVisibility` (`self.Interact Text1`) false false)
    (set `self.Strength Puzzle` false)))

(fn `UserConstructionScript`)