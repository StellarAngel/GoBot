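; BP_Door is a door actor that slides open with an unlock sound when Openingdoor_Event fires.
; The event ignores its Index input, instead finding its own position among all BP_Door actors.
; The doors at array positions one and two run separate timelines, moving along Y or Z respectively with hardcoded coordinates on the other axes.
; UnlockDoor plays on every timeline update, not once.
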(event `self.ReceiveTick`
  (params (DeltaSeconds :type "Float (single-precision)")))

(event `Opening door_Event`
  (params (Index :type Integer))
  (bind _outactors (`GameplayStatics.GetAllActorsOfClass` "BP_Door_C"))
  (for (_array_element _array_index) _outactors
    (if (and (== 1 _array_index) (== self _array_element))
      (bind (_direction _newtrack_0) (`Timeline|Timeline` :!via `PlayFromStart`)
        (:`Update`
          (`self.K2_SetActorRelativeLocation` (`KismetMathLibrary.MakeVector` -3217.010305 _newtrack_0 235.809559))
          (`GameplayStatics.PlaySound2D` "/Game/Audio/UnlockDoor.UnlockDoor" 1.0 1.0 0.0 null null)))
      (elif (and (== _array_index 2) (== self _array_element))
        (bind (_direction_2 _newtrack_0_2) (`Timeline|Timeline_0` :!via `PlayFromStart`)
          (:`Update`
            (`self.K2_SetActorRelativeLocation` (`KismetMathLibrary.MakeVector` 5237.124513 -4479.062814 _newtrack_0_2))
            (`GameplayStatics.PlaySound2D` "/Game/Audio/UnlockDoor.UnlockDoor" 1.0 1.0 0.0 null null)))))))

(fn `UserConstructionScript`)