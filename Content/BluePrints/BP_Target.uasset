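; Shootable puzzle target that rewards the player when the last target in its numbered puzzle group is destroyed.
; A BP_Bullet overlapping the Box destroys both actors with a sound, then recounts remaining BP_Target actors sharing the PuzzleNumber.
; An empty group grants the first-person character a ticket, or the diamond or ruby flag for the last two puzzles.
; Each puzzle number has its own duplicated branch, using GetAllActorsOfClass scans.
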(event `self.ReceiveBeginPlay`)

(event `self.ReceiveTick`
  (params (DeltaSeconds :type "Float (single-precision)")))

(event `self.Box.OnComponentBeginOverlap`
  (params (OverlappedComponent :type "PrimitiveComponent Object Reference") (OtherActor :type "Actor Object Reference") (OtherComp :type "PrimitiveComponent Object Reference") (OtherBodyIndex :type Integer) (bFromSweep :type Boolean) (SweepResult :type "HitResult Structure (by ref)"))
  (bind _outactors (`GameplayStatics.GetAllActorsOfClass` "/Game/Projectiles/BP_Bullet.BP_Bullet_C"))
  (for _array_element _outactors
    (if (== _array_element OtherActor)
      (bind _asbp_bullet (cast `/Game/Projectiles/BP_Bullet` _array_element))
      (bind _output_get (set `self.Bullet Ref` _asbp_bullet))
      (`self.K2_DestroyActor` _output_get)
      (`GameplayStatics.PlaySound2D` "/Game/Audio/DartShoot_Cue.DartShoot_Cue" 1.0 1.0 0.0 null null)
      (if (== (`self.Puzzle Number`) 1)
        (set `self.puzzle1 Target  Count` 0)
        (`self.K2_DestroyActor`)
        (`GameplayStatics.PlaySound2D` "/Game/Audio/DartShoot_Cue.DartShoot_Cue" 1.0 1.0 0.0 null null)
        (bind _outactors_2 (`GameplayStatics.GetAllActorsOfClass` "BP_Target_C"))
        (for _array_element_2 _outactors_2
          (if (== (`/Game/BluePrints/BP_Target.Puzzle Number` _array_element_2) 1)
            (set `self.puzzle1 Target  Count` (+ (`self.puzzle1 Target  Count`) 1))))
        (if (== (`self.puzzle1 Target  Count`) 0)
          (bind _asbp_first_person_character (cast `/Game/FirstPerson/Blueprints/BP_FirstPersonCharacter` (`GameplayStatics.GetPlayerCharacter` 0)))
          (set `/Game/FirstPerson/Blueprints/BP_FirstPersonCharacter.Tickets` (+ (`/Game/FirstPerson/Blueprints/BP_FirstPersonCharacter.Tickets` _asbp_first_person_character) 1.0) _asbp_first_person_character))
        (elif (== (`self.Puzzle Number`) 2)
          (set `self.Puzzle2 Target Count` 0)
          (`self.K2_DestroyActor`)
          (`GameplayStatics.PlaySound2D` "/Game/Audio/DartShoot_Cue.DartShoot_Cue" 1.0 1.0 0.0 null null)
          (bind _outactors_3 (`GameplayStatics.GetAllActorsOfClass` "BP_Target_C"))
          (for _array_element_3 _outactors_3
            (if (== (`/Game/BluePrints/BP_Target.Puzzle Number` _array_element_3) 2)
              (set `self.Puzzle2 Target Count` (+ (`self.Puzzle2 Target Count`) 1))))
          (if (== (`self.Puzzle2 Target Count`) 0)
            (bind _asbp_first_person_character_2 (cast `/Game/FirstPerson/Blueprints/BP_FirstPersonCharacter` (`GameplayStatics.GetPlayerCharacter` 0)))
            (set `/Game/FirstPerson/Blueprints/BP_FirstPersonCharacter.Tickets` (+ (`/Game/FirstPerson/Blueprints/BP_FirstPersonCharacter.Tickets` _asbp_first_person_character_2) 1.0) _asbp_first_person_character_2))
          (elif (== (`self.Puzzle Number`) 3)
            (set `self.Puzzle3 Target Count` 0)
            (`self.K2_DestroyActor`)
            (`GameplayStatics.PlaySound2D` "/Game/Audio/DartShoot_Cue.DartShoot_Cue" 1.0 1.0 0.0 null null)
            (bind _outactors_4 (`GameplayStatics.GetAllActorsOfClass` "BP_Target_C"))
            (for _array_element_4 _outactors_4
              (if (== (`/Game/BluePrints/BP_Target.Puzzle Number` _array_element_4) 3)
                (set `self.Puzzle3 Target Count` (+ (`self.Puzzle3 Target Count`) 1))))
            (if (== (`self.Puzzle3 Target Count`) 0)
              (bind _asbp_first_person_character_3 (cast `/Game/FirstPerson/Blueprints/BP_FirstPersonCharacter` (`GameplayStatics.GetPlayerCharacter` 0)))
              (set `/Game/FirstPerson/Blueprints/BP_FirstPersonCharacter.Tickets` (+ (`/Game/FirstPerson/Blueprints/BP_FirstPersonCharacter.Tickets` _asbp_first_person_character_3) 1.0) _asbp_first_person_character_3))
            (elif (== (`self.Puzzle Number`) 4)
              (set `self.Puzzle4 Target Count` 0)
              (`self.K2_DestroyActor`)
              (`GameplayStatics.PlaySound2D` "/Game/Audio/DartShoot_Cue.DartShoot_Cue" 1.0 1.0 0.0 null null)
              (bind _outactors_5 (`GameplayStatics.GetAllActorsOfClass` "BP_Target_C"))
              (for _array_element_5 _outactors_5
                (if (== (`/Game/BluePrints/BP_Target.Puzzle Number` _array_element_5) 4)
                  (set `self.Puzzle4 Target Count` (+ (`self.Puzzle4 Target Count`) 1))))
              (if (== (`self.Puzzle4 Target Count`) 0)
                (bind _asbp_first_person_character_4 (cast `/Game/FirstPerson/Blueprints/BP_FirstPersonCharacter` (`GameplayStatics.GetPlayerCharacter` 0)))
                (set `/Game/FirstPerson/Blueprints/BP_FirstPersonCharacter.Tickets` (+ (`/Game/FirstPerson/Blueprints/BP_FirstPersonCharacter.Tickets` _asbp_first_person_character_4) 1.0) _asbp_first_person_character_4))
              (elif (== (`self.Puzzle Number`) 5)
                (set `self.Puzzle5TargetCount` 0)
                (`self.K2_DestroyActor`)
                (`GameplayStatics.PlaySound2D` "/Game/Audio/DartShoot_Cue.DartShoot_Cue" 1.0 1.0 0.0 null null)
                (bind _outactors_6 (`GameplayStatics.GetAllActorsOfClass` "BP_Target_C"))
                (for _array_element_6 _outactors_6
                  (if (== (`/Game/BluePrints/BP_Target.Puzzle Number` _array_element_6) 5)
                    (set `self.Puzzle5TargetCount` (+ (`self.Puzzle5TargetCount`) 1))))
                (if (== (`self.Puzzle5TargetCount`) 0)
                  (bind _asbp_first_person_character_5 (cast `/Game/FirstPerson/Blueprints/BP_FirstPersonCharacter` (`GameplayStatics.GetPlayerCharacter` 0)))
                  (set `/Game/FirstPerson/Blueprints/BP_FirstPersonCharacter.Tickets` (+ (`/Game/FirstPerson/Blueprints/BP_FirstPersonCharacter.Tickets` _asbp_first_person_character_5) 1.0) _asbp_first_person_character_5))
                (elif (== (`self.Puzzle Number`) 6)
                  (set `self.Puzzle6 Target Count` 0)
                  (`self.K2_DestroyActor`)
                  (`GameplayStatics.PlaySound2D` "/Game/Audio/DartShoot_Cue.DartShoot_Cue" 1.0 1.0 0.0 null null)
                  (bind _outactors_7 (`GameplayStatics.GetAllActorsOfClass` "BP_Target_C"))
                  (for _array_element_7 _outactors_7
                    (if (== (`/Game/BluePrints/BP_Target.Puzzle Number` _array_element_7) 6)
                      (set `self.Puzzle6 Target Count` (+ (`self.Puzzle6 Target Count`) 1))))
                  (if (== (`self.Puzzle6 Target Count`) 0)
                    (bind _asbp_first_person_character_6 (cast `/Game/FirstPerson/Blueprints/BP_FirstPersonCharacter` (`GameplayStatics.GetPlayerCharacter` 0)))
                    (set `/Game/FirstPerson/Blueprints/BP_FirstPersonCharacter.HasDiamond` true _asbp_first_person_character_6))
                  (elif (== (`self.Puzzle Number`) 7)
                    (set `self.Puzzle7 Target Count` 0)
                    (`self.K2_DestroyActor`)
                    (`GameplayStatics.PlaySound2D` "/Game/Audio/DartShoot_Cue.DartShoot_Cue" 1.0 1.0 0.0 null null)
                    (bind _outactors_8 (`GameplayStatics.GetAllActorsOfClass` "BP_Target_C"))
                    (for _array_element_8 _outactors_8
                      (if (== (`/Game/BluePrints/BP_Target.Puzzle Number` _array_element_8) 7)
                        (set `self.Puzzle7 Target Count` (+ (`self.Puzzle7 Target Count`) 1))))
                    (if (== (`self.Puzzle7 Target Count`) 0)
                      (bind _asbp_first_person_character_7 (cast `/Game/FirstPerson/Blueprints/BP_FirstPersonCharacter` (`GameplayStatics.GetPlayerCharacter` 0)))
                      (set `/Game/FirstPerson/Blueprints/BP_FirstPersonCharacter.HasRuby` true _asbp_first_person_character_7))))))))))))

(fn `UserConstructionScript`)