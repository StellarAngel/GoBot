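; Dialogue component that shows one line of data-table-driven dialogue in a UI widget each time its Ineract event fires.
; It looks up the current row, creates a new widget with the speaker name and line, and adds it to the viewport.
; The row then supplies the next row, table and end-of-dialogue flag, chaining lines across calls.
; The flag is only stored here, and a leftover debug print runs on every interaction.
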(event `/Game/Dialogue/BP_Interact.Ineract`
  (params (playerRef :type "/Game/FirstPerson/Blueprints/BP_FirstPersonCharacter Object Reference"))
  (`KismetSystemLibrary.PrintString` "im gonna fucking kms")
  (bind _returnvalue (`|GetDataTableRow` (`self.Data Table`) (`self.Row Name`))
    (:`then`
      (bind (_dialogue _row _datatable _enddialogue) (break `/Game/Dialogue/DialogueStructure` _returnvalue))
      (bind _returnvalue_2 (`|CreateWidget` "/Game/Dialogue/UI_Dialogue.UI_Dialogue_C" null (`KismetTextLibrary.Conv_NameToText` (`self.Name`)) _dialogue))
      (bind _output_get (set `self.DialogueWidget` _returnvalue_2))
      (`UserWidget.AddToViewport` _output_get 0)
      (set `self.Row Name` _row)
      (set `self.Data Table` _datatable)
      (set `self.EndDialogue` _enddialogue))))